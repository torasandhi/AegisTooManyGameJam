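; BP_Tile_3 is a world tile with three child-actor obstacles that slide sideways as the character passes through.
; The Start overlap reveals them, and SetUpObstacle gives each a random type, mesh, move duration and Left or Right start, then registers it with the game mode.
; MoveComponentTo slides each to the opposite side, and IStop halts one by name.
; The End overlap notifies the game mode for removal and hides them.
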(event `self.IStop`
  (params (Name :type String))
  (switch `string` Name
    (:`ChildActor1`
      (goto _label :!via `Stop`))
    (:`ChildActor2`
      (goto _label_2 :!via `Stop`))
    (:`ChildActor3`
      (goto _label_3 :!via `Stop`))))

(event `self.Start.OnComponentBeginOverlap`
  (params (OverlappedComponent :type "PrimitiveComponent Object Reference") (OtherActor :type "Actor Object Reference") (OtherComp :type "PrimitiveComponent Object Reference") (OtherBodyIndex :type Integer) (bFromSweep :type Boolean) (SweepResult :type "HitResult Structure (by ref)"))
  (if (`self.ActorHasTag` OtherActor "Character")
    (`SceneComponent.SetHiddenInGame` (`self.ChildActor1`) false false)
    (`SceneComponent.SetHiddenInGame` (`self.ChildActor2`) false false)
    (`SceneComponent.SetHiddenInGame` (`self.ChildActor3`) false false)
    (`|ExecutionSequence`
      (:`then_0`
        (bind (_returnlocation _returnspeed) (`self.SetUpObstacle` (`self.ChildActor1`)))
        (`KismetSystemLibrary.MoveComponentTo` (`self.ChildActor1`) _returnlocation (struct) false false _returnspeed :!label _label))
      (:`then_1`
        (bind (_returnlocation_2 _returnspeed_2) (`self.SetUpObstacle` (`self.ChildActor2`)))
        (`KismetSystemLibrary.MoveComponentTo` (`self.ChildActor2`) _returnlocation_2 (struct) false false _returnspeed_2 :!label _label_2))
      (:`then_2`
        (bind (_returnlocation_3 _returnspeed_3) (`self.SetUpObstacle` (`self.ChildActor3`)))
        (`KismetSystemLibrary.MoveComponentTo` (`self.ChildActor3`) _returnlocation_3 (struct) false false _returnspeed_3 :!label _label_3)))))

(event `self.End.OnComponentBeginOverlap`
  (params (OverlappedComponent :type "PrimitiveComponent Object Reference") (OtherActor :type "Actor Object Reference") (OtherComp :type "PrimitiveComponent Object Reference") (OtherBodyIndex :type Integer) (bFromSweep :type Boolean) (SweepResult :type "HitResult Structure (by ref)"))
  (if (`self.ActorHasTag` OtherActor "Character")
    (message `/Game/Interaface/BPI_GameMode.IRemoveArray` (`GameplayStatics.GetGameMode`) self)
    (`SceneComponent.SetHiddenInGame` (`self.ChildActor1`) true false)
    (`SceneComponent.SetHiddenInGame` (`self.ChildActor2`) true false)
    (`SceneComponent.SetHiddenInGame` (`self.ChildActor3`) true false)))

(fn `GetWorld`
  (params (Target :type "Object Object Reference"))
  (returns (World :type String))
  (bind _world (message `/Game/Interaface/BPI_Obstacle.IGetWorld` Target))
  (return _world))

(fn `SetUpObstacle`
  (params (Target :type "ChildActorComponent Object Reference"))
  (returns (ReturnLocation :type "Vector Structure") (ReturnSpeed :type "Float (double-precision)"))
  (locals (Speed :type "Float (double-precision)") (ObstacleType :type Integer) (Index :type Integer))
  (bind _obstacletype (`local.ObstacleType`))
  (bind (_returnvalue_x _returnvalue_y) (`KismetMathLibrary.BreakVector` (`self.TargetB` (`local.Index`))))
  (bind (_returnvalue_x_2 _returnvalue_y_2) (`KismetMathLibrary.BreakVector` (`self.TargetA` (`local.Index`))))
  (bind (_relativelocation_x _relativelocation_y _relativelocation_z) (`KismetMathLibrary.BreakVector` (`SceneComponent.RelativeLocation` (`local.Target`))))
  (bind (_relativelocation_x_2 _relativelocation_y_2 _relativelocation_z_2) (`KismetMathLibrary.BreakVector` (`SceneComponent.RelativeLocation` (`local.Target`))))
  (set `local.ObstacleType` (`KismetMathLibrary.RandomIntegerInRange` 0 3))
  (set `local.Speed` (select `int` (`local.ObstacleType`) :`0` 10.0 :`1` 13.0 :`2` 9.0 :`3` 11.0))
  (message `/Game/Interaface/BPI_Obstacle.ISetMesh` (`ChildActorComponent.ChildActor` (`local.Target`)) (select `int` _obstacletype :`0` "/ControlRig/Controls/ControlRig_Box_solid.ControlRig_Box_solid" :`1` "/Engine/VREditor/TransformGizmo/RotationHandleFull.RotationHandleFull" :`2` "/Engine/BasicShapes/Cone.Cone" :`3` "/Engine/BasicShapes/Cylinder.Cylinder" :!type "StaticMesh Object Reference") _obstacletype)
  (set `local.Index` (`KismetMathLibrary.RandomIntegerInRange` 0 1))
  (`SceneComponent.K2_SetRelativeLocation` (`local.Target`) (`KismetMathLibrary.MakeVector` _relativelocation_x_2 _returnvalue_y _relativelocation_z_2) false false)
  (message `/Game/Interaface/BPI_GameMode.IAddObstacle` (`GameplayStatics.GetGameMode`) (`ChildActorComponent.ChildActor` (`local.Target`)))
  (return (`KismetMathLibrary.MakeVector` _relativelocation_x _returnvalue_y_2 _relativelocation_z) (`local.Speed`)))

(fn `TargetA`
  (params (Index :type Integer))
  (returns (ReturnValue :type "Vector Structure"))
  (return (select `int` Index :`0` (`SceneComponent.RelativeLocation` (`self.Right`)) :`1` (`SceneComponent.RelativeLocation` (`self.Left`)))))

(fn `TargetB`
  (params (Index :type Integer))
  (returns (ReturnValue :type "Vector Structure"))
  (return (select `int` Index :`0` (`SceneComponent.RelativeLocation` (`self.Left`)) :`1` (`SceneComponent.RelativeLocation` (`self.Right`)))))

(fn `UserConstructionScript`)