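; World tile that launches two moving obstacles across the track when a tagged Character enters its Start trigger.
; SetUpObstacle randomizes each child actor's mesh, speed and starting side, turns it by a cross-product test and registers it with the GameMode.
; MoveComponentTo slides each across; IStop halts one by name, and leaving Start sends both IEmptyMessage.
; The End trigger is empty, and the hide and deregistration nodes are disconnected.
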(event `/Game/Interaface/BPI_Tile.IStop`
  (params (Name :type String))
  (switch `string` Name
    (:`ChildActor1`
      (goto _label :!via `Stop`))
    (:`ChildActor2`
      (goto _label_2 :!via `Stop`))))

(event `self.Start.OnComponentBeginOverlap`
  (params (OverlappedComponent :type "PrimitiveComponent Object Reference") (OtherActor :type "Actor Object Reference") (OtherComp :type "PrimitiveComponent Object Reference") (OtherBodyIndex :type Integer) (bFromSweep :type Boolean) (SweepResult :type "HitResult Structure (by ref)"))
  (if (`self.ActorHasTag` OtherActor "Character")
    (`SceneComponent.SetHiddenInGame` (`self.ChildActor1`) false false)
    (`SceneComponent.SetHiddenInGame` (`self.ChildActor2`) false false)
    (`|ExecutionSequence`
      (:`then_0`
        (bind (_returnlocation _returnspeed) (`self.SetUpObstacle` (`self.ChildActor1`)))
        (`KismetSystemLibrary.MoveComponentTo` (`self.ChildActor1`) _returnlocation (`SceneComponent.RelativeRotation` (`self.ChildActor1`)) false false _returnspeed :!label _label))
      (:`then_1`
        (bind (_returnlocation_2 _returnspeed_2) (`self.SetUpObstacle` (`self.ChildActor2`)))
        (`KismetSystemLibrary.MoveComponentTo` (`self.ChildActor2`) _returnlocation_2 (`SceneComponent.RelativeRotation` (`self.ChildActor2`)) false false _returnspeed_2 :!label _label_2)))))

(event `self.End.OnComponentBeginOverlap`
  (params (OverlappedComponent :type "PrimitiveComponent Object Reference") (OtherActor :type "Actor Object Reference") (OtherComp :type "PrimitiveComponent Object Reference") (OtherBodyIndex :type Integer) (bFromSweep :type Boolean) (SweepResult :type "HitResult Structure (by ref)")))

(event `self.Start.OnComponentEndOverlap`
  (params (OverlappedComponent :type "PrimitiveComponent Object Reference") (OtherActor :type "Actor Object Reference") (OtherComp :type "PrimitiveComponent Object Reference") (OtherBodyIndex :type Integer))
  (if (`self.ActorHasTag` OtherActor "Character")
    (message `/Game/Interaface/BPI_Obstacle.IEmpty` (`ChildActorComponent.ChildActor` (`self.ChildActor1`)))
    (message `/Game/Interaface/BPI_Obstacle.IEmpty` (`ChildActorComponent.ChildActor` (`self.ChildActor2`)))))

(fn `Cross`
  (params (A :type "Vector Structure"))
  (returns (ReturnValue :type "Float (double-precision)"))
  (bind (_returnvalue_x _returnvalue_y _returnvalue_z) (`KismetMathLibrary.BreakVector` (`KismetMathLibrary.Normal` (`KismetMathLibrary.Cross_VectorVector` A (`self.GetActorForwardVector`)))))
  (return (* _returnvalue_z 180.0)))

(fn `GetWorld`
  (params (Target :type "Object Object Reference"))
  (returns (World :type String))
  (bind _world (message `/Game/Interaface/BPI_Obstacle.IGetWorld` Target))
  (return _world))

(fn `SetUpObstacle`
  (params (Target :type "ChildActorComponent Object Reference"))
  (returns (ReturnLocation :type "Vector Structure") (ReturnSpeed :type "Float (double-precision)"))
  (locals (Speed :type "Float (double-precision)") (ObstacleType :type Integer) (Index :type Integer))
  (bind _obstacletype (`local.ObstacleType`))
  (bind (_returnvalue_x _returnvalue_y) (`KismetMathLibrary.BreakVector` (`self.TargetB` (`local.Index`))))
  (bind (_returnvalue_x_2 _returnvalue_y_2) (`KismetMathLibrary.BreakVector` (`self.TargetA` (`local.Index`))))
  (bind _childactor (`ChildActorComponent.ChildActor` (`local.Target`)))
  (bind (_relativelocation_x _relativelocation_y _relativelocation_z) (`KismetMathLibrary.BreakVector` (`SceneComponent.RelativeLocation` (`local.Target`))))
  (bind (_relativelocation_x_2 _relativelocation_y_2 _relativelocation_z_2) (`KismetMathLibrary.BreakVector` (`SceneComponent.RelativeLocation` (`local.Target`))))
  (bind _returnvalue (`KismetMathLibrary.MakeVector` _relativelocation_x _returnvalue_y_2 _relativelocation_z))
  (set `local.ObstacleType` (`KismetMathLibrary.RandomIntegerInRange` 0 3))
  (set `local.Speed` (select `int` (`local.ObstacleType`) :`0` 12.0 :`1` 15.0 :`2` 11.0 :`3` 13.0))
  (message `/Game/Interaface/BPI_Obstacle.ISetMesh` (`ChildActorComponent.ChildActor` (`local.Target`)) (select `int` _obstacletype :`0` "/Game/Assets/Obstacle/motor_finish.motor_finish" :`1` "/Game/Assets/Obstacle/car/CarModel1.CarModel1" :`2` "/Game/Assets/Obstacle/vehicle_gimjam.vehicle_gimjam" :`3` "/Engine/BasicShapes/Cylinder.Cylinder" :!type "StaticMesh Object Reference") _obstacletype)
  (set `local.Index` (`KismetMathLibrary.RandomIntegerInRange` 0 1))
  (`SceneComponent.K2_SetRelativeLocation` (`local.Target`) (`KismetMathLibrary.MakeVector` _relativelocation_x_2 _returnvalue_y _relativelocation_z_2) false false)
  (message `/Game/Interaface/BPI_Obstacle.IAddWorlds` _childactor)
  (message `/Game/Interaface/BPI_GameMode.IAddObstacle` (`GameplayStatics.GetGameMode`) _childactor)
  (`SceneComponent.K2_SetRelativeRotation` (`local.Target`) (`KismetMathLibrary.MakeRotator` 0.0 0.0 (`KismetMathLibrary.SelectFloat` 180.0 0.0 (> (`self.Cross` _returnvalue) 0.0))) false false)
  (return _returnvalue (`local.Speed`)))

(fn `TargetA`
  (params (Index :type Integer))
  (returns (ReturnValue :type "Vector Structure"))
  (return (select `int` Index :`0` (`SceneComponent.RelativeLocation` (`self.Right`)) :`1` (`SceneComponent.RelativeLocation` (`self.Left`)))))

(fn `TargetB`
  (params (Index :type Integer))
  (returns (ReturnValue :type "Vector Structure"))
  (return (select `int` Index :`0` (`SceneComponent.RelativeLocation` (`self.Left`)) :`1` (`SceneComponent.RelativeLocation` (`self.Right`)))))

(fn `UserConstructionScript`)