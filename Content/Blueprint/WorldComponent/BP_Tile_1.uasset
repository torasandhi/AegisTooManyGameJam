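; World tile that spawns a randomized obstacle crossing from one side to the other when a Character-tagged actor enters its Start trigger.
; SetUpObstacle picks type, mesh, travel time and starting side, then registers the ChildActor obstacle with the GameMode through interface messages.
; A MoveComponentTo slides the obstacle to the opposite side until finished or halted by IStop.
; Leaving Start sends the obstacle IEmptyMessage; GameMode removal calls exist but are unconnected.
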(event `self.Start.OnComponentBeginOverlap`
  (params (OverlappedComponent :type "PrimitiveComponent Object Reference") (OtherActor :type "Actor Object Reference") (OtherComp :type "PrimitiveComponent Object Reference") (OtherBodyIndex :type Integer) (bFromSweep :type Boolean) (SweepResult :type "HitResult Structure (by ref)"))
  (if (`self.ActorHasTag` OtherActor "Character")
    (`SceneComponent.SetHiddenInGame` (`self.ChildActor`) false false)
    (bind (_returnlocation _returnspeed) (`self.SetUpObstacle`))
    (`KismetSystemLibrary.MoveComponentTo` (`self.ChildActor`) _returnlocation (struct) false false _returnspeed :!label _label)))

(event `/Game/Interaface/BPI_Tile.IStop`
  (params (Name :type String))
  (goto _label :!via `Stop`))

(event `self.End.OnComponentBeginOverlap`
  (params (OverlappedComponent :type "PrimitiveComponent Object Reference") (OtherActor :type "Actor Object Reference") (OtherComp :type "PrimitiveComponent Object Reference") (OtherBodyIndex :type Integer) (bFromSweep :type Boolean) (SweepResult :type "HitResult Structure (by ref)")))

(event `self.Start.OnComponentEndOverlap`
  (params (OverlappedComponent :type "PrimitiveComponent Object Reference") (OtherActor :type "Actor Object Reference") (OtherComp :type "PrimitiveComponent Object Reference") (OtherBodyIndex :type Integer))
  (if (`self.ActorHasTag` OtherActor "Character")
    (message `/Game/Interaface/BPI_Obstacle.IEmpty` (`ChildActorComponent.ChildActor` (`self.ChildActor`)))))

(fn `GetWorld`
  (params (Target :type "Object Object Reference"))
  (returns (World :type String))
  (bind _world (message `/Game/Interaface/BPI_Obstacle.IGetWorld` Target))
  (return _world))

(fn `SetUpObstacle`
  (returns (ReturnLocation :type "Vector Structure") (ReturnSpeed :type "Float (double-precision)"))
  (locals (Speed :type "Float (double-precision)") (ObstacleType :type Integer) (Index :type Integer))
  (bind _obstacletype (`local.ObstacleType`))
  (bind _childactor (`ChildActorComponent.ChildActor` (`self.ChildActor`)))
  (set `local.ObstacleType` (`KismetMathLibrary.RandomIntegerInRange` 0 3))
  (set `local.Speed` (select `int` (`local.ObstacleType`) :`0` 12.0 :`1` 15.0 :`2` 11.0 :`3` 13.0))
  (message `/Game/Interaface/BPI_Obstacle.ISetMesh` (`ChildActorComponent.ChildActor` (`self.ChildActor`)) (select `int` _obstacletype :`0` "/Game/Assets/Obstacle/motor_finish.motor_finish" :`1` "/Game/Assets/Obstacle/motor_finish.motor_finish" :`2` "/Game/Assets/Obstacle/vehicle_gimjam.vehicle_gimjam" :`3` "/Engine/BasicShapes/Cylinder.Cylinder" :!type "StaticMesh Object Reference") _obstacletype)
  (set `local.Index` (`KismetMathLibrary.RandomIntegerInRange` 0 1))
  (`SceneComponent.K2_SetRelativeLocation` (`self.ChildActor`) (`self.TargetB` (`local.Index`)) false false)
  (message `/Game/Interaface/BPI_Obstacle.IAddWorlds` _childactor)
  (message `/Game/Interaface/BPI_GameMode.IAddObstacle` (`GameplayStatics.GetGameMode`) _childactor)
  (return (`self.TargetA` (`local.Index`)) (`local.Speed`)))

(fn `TargetA`
  (params (Index :type Integer))
  (returns (ReturnValue :type "Vector Structure"))
  (return (select `int` Index :`0` (`SceneComponent.RelativeLocation` (`self.Right`)) :`1` (`SceneComponent.RelativeLocation` (`self.Left`)))))

(fn `TargetB`
  (params (Index :type Integer))
  (returns (ReturnValue :type "Vector Structure"))
  (return (select `int` Index :`0` (`SceneComponent.RelativeLocation` (`self.Left`)) :`1` (`SceneComponent.RelativeLocation` (`self.Right`)))))

(fn `UserConstructionScript`)