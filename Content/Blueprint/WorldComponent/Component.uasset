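; Obstacle actor that slides between side markers, carries a word ("World") on a widget and shows the HUD finish menu when hit by a Character.
; IAddWorlds picks a random word with a first letter unlike those from the GameMode, and IUpdateWorld highlights it in rich text.
; IStop clears the text and pauses movement for five seconds.
; The distance-based show/hide logic that randomizes mesh, speed and side is disconnected.
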(event `self.ReceiveTick`
  (params (DeltaSeconds :type "Float (single-precision)")))

(event `EMoveing`
  (bind _returnvalue (`self.TargetA`))
  (`KismetSystemLibrary.MoveComponentTo` (`self.Obstacle`) _returnvalue (struct) false false (`self.Speed`) :!label _label)
  (if (== (`SceneComponent.RelativeLocation` (`self.Obstacle`)) _returnvalue)
    (`SceneComponent.K2_SetRelativeLocation` (`self.Obstacle`) (`self.TargetB`) false false)
    (goto _label)))

(event `/Game/Interaface/BPI_Obstacle.IStop`
  (message `/Game/Interaface/BPIW_World.ISetText` (`WidgetComponent.GetWidget` (`self.Widget`)) "")
  (`KismetSystemLibrary.K2_SetTimerDelegate` (delegate `EMove`) 5.0)
  (goto _label :!via `Stop`))

(event `EMove`
  (goto _label))

(event `/Game/Interaface/BPI_Obstacle.IUpdateWorld`
  (params (CurrentWorld :type String))
  (`self.HighlightWorld` CurrentWorld))

(event `self.Obstacle.OnComponentBeginOverlap`
  (params (OverlappedComponent :type "PrimitiveComponent Object Reference") (OtherActor :type "Actor Object Reference") (OtherComp :type "PrimitiveComponent Object Reference") (OtherBodyIndex :type Integer) (bFromSweep :type Boolean) (SweepResult :type "HitResult Structure (by ref)"))
  (if (`self.ActorHasTag` OtherActor "Character")
    (message `/Game/Interaface/BPI_HUD.IFinishMenu` (`PlayerController.GetHUD` (`GameplayStatics.GetPlayerController` 0)) true)))

(event `/Game/Interaface/BPI_Obstacle.IAddWorlds`
  (bind _result (`self.CheckAndSetWorld`))
  (message `/Game/Interaface/BPIW_World.ISetText` (`WidgetComponent.GetWidget` (`self.Widget`)) (`KismetTextLibrary.Conv_StringToText` _result)))

(fn `CheckAndSetWorld`
  (returns (Result :type String))
  (locals (World :type String))
  (bind _output_get (`self.SetWorld` :!label _label))
  (set `local.World` _output_get)
  (if (`self.CheckWorld`)
    (return (`local.World`))
    (else
      (goto _label))))

(fn `CheckFirstWorld`
  (params (SourceString :type String))
  (returns (ReturnValue :type Boolean))
  (return (`KismetStringLibrary.NotEqual_StrStr` (`KismetStringLibrary.Left` SourceString 1) (`KismetStringLibrary.Left` (`self.World`) 1))))

(fn `CheckWorld`
  (returns (Value :type Boolean))
  (locals (RetValue :type Boolean))
  (if (`self.LengthWorld` (`self.GetWorlds`))
    (for _array_element (`self.GetWorlds`)
      (bind _output_get (set `local.RetValue` (`self.CheckFirstWorld` _array_element)))
      (if (not _output_get)
        (return (`local.RetValue`))))
    (return (`local.RetValue`))
    (else
      (bind _output_get_2 (set `local.RetValue` true))
      (return _output_get_2))))

(fn `GetLenWorld`
  (params (World :type String))
  (returns (Len :type Integer))
  (return (- (`KismetStringLibrary.Len` World) 1)))

(fn `GetListWorlds`
  (returns (Worlds :type "Array of String"))
  (bind _worlds (message `/Game/Interaface/BPI_Instance.IGetWorlds` (`GameplayStatics.GetGameInstance`) (`self.ObstacleType`)))
  (return _worlds))

(fn `GetWorlds`
  (returns (Worlds :type "Array of String"))
  (bind _worlds (message `/Game/Interaface/BPI_GameMode.IGetWorlds` (`GameplayStatics.GetGameMode`)))
  (return _worlds))

(fn `HighlightWorld`
  (params (CurrentWorld :type String))
  (message `/Game/Interaface/BPIW_World.ISetText` (`WidgetComponent.GetWidget` (`self.Widget`)) (`self.SelectionWorld` CurrentWorld CurrentWorld)))

(fn `IGetWorld`
  (returns (World :type String))
  (return (`self.World`)))

(fn `LengthWorld`
  (params (TargetArray :type "Array of String (by ref)"))
  (returns (ReturnValue :type Boolean))
  (return (> (`KismetArrayLibrary.Array_Length` TargetArray) 0)))

(fn `SelectionWorld`
  (params (World :type String) (B :type String))
  (returns (ReturnValue :type Text))
  (bind _world (`self.World`))
  (return (`KismetTextLibrary.Conv_StringToText` (`KismetStringLibrary.Concat_StrStr` (`KismetStringLibrary.Concat_StrStr` "<True>" B "</>") (`KismetStringLibrary.Right` _world (- (`KismetStringLibrary.Len` _world) (+ (`self.GetLenWorld` World) 1)))))))

(fn `SetWorld`
  (returns (Output_Get :type String))
  (bind _worlds (`self.GetListWorlds`))
  (bind _output_get (set `self.World` (`|GetArrayItem` _worlds (`KismetMathLibrary.RandomIntegerInRange` 0 (- (`KismetArrayLibrary.Array_Length` _worlds) 1)))))
  (return _output_get))

(fn `TargetA`
  (returns (ReturnValue :type "Vector Structure"))
  (return (select `int` (`self.Index`) :`0` (`SceneComponent.RelativeLocation` (`self.Right`)) :`1` (`SceneComponent.RelativeLocation` (`self.Left`)))))

(fn `TargetB`
  (returns (ReturnValue :type "Vector Structure"))
  (return (select `int` (`self.Index`) :`0` (`SceneComponent.RelativeLocation` (`self.Left`)) :`1` (`SceneComponent.RelativeLocation` (`self.Right`)))))

(fn `UserConstructionScript`)