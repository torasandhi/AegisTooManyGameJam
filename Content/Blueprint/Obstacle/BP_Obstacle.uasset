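; Vehicle obstacle, placed as a child actor, that shows a word ("World") and ends the game with a crash sound, finish menu and pause when it hits the Character.
; An index set with the mesh selects material, one-shot delayed horn and word list.
; Random words are redrawn until their first letter is unique among active words.
; Interface events highlight the word via rich-text tags or clear and deregister it.
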(event `/Game/Interaface/BPI_Obstacle.ISetMesh`
  (params (Mesh :type "StaticMesh Object Reference") (Index :type Integer))
  (`StaticMeshComponent.SetStaticMesh` (`self.Cube`) Mesh)
  (bind _output_get (set `self.Index` Index))
  (set `self.bIsUpdateWorld` false)
  (`PrimitiveComponent.SetMaterial` (`self.Cube`) 0 (select `int` Index :`0` "/Game/Assets/Obstacle/motor.motor" :`1` "/Game/Assets/Obstacle/motor.motor" :`2` "/Game/Assets/Obstacle/truck.truck" :`3` null :!type "MaterialInterface Object Reference"))
  (bind _returnvalue (`KismetSystemLibrary.K2_SetTimerDelegate` (delegate `PlaySFX`) (`KismetMathLibrary.RandomFloatInRange` 1.0 3.0) true))
  (set `self.TimerSoundKlakson` _returnvalue))

(event `PlaySFX`
  (`GameplayStatics.PlaySound2D` (select `int` (stale `/Game/Interaface/BPI_Obstacle.ISetMesh` _output_get) :`0` "/Game/Sound/Klakson_Motor.Klakson_Motor" :`1` "/Game/Sound/Klakson_Mobil.Klakson_Mobil" :`2` "/Game/Sound/Klakson_Mobil.Klakson_Mobil" :`3` "/Game/Sound/Klakson_Mobil.Klakson_Mobil" :!type "SoundBase Object Reference") 1.0 1.0 0.0 null null)
  (`KismetSystemLibrary.K2_ClearAndInvalidateTimerHandle` (`self.TimerSoundKlakson`)))

(event `/Game/Interaface/BPI_Obstacle.IPlay`
  (params (Location :type "Vector Structure") (Speed :type "Float (double-precision)")))

(event `/Game/Interaface/BPI_Obstacle.IStop`
  (bind _returnvalue (`GameplayStatics.GetGameMode`))
  (message `/Game/Interaface/BPI_Tile.IStop` (`self.GetParentActor`) (`KismetSystemLibrary.GetObjectName` (`self.GetParentComponent`)))
  (message `/Game/Interaface/BPIW_World.ISetText` (`WidgetComponent.GetWidget` (`self.Widget`)) "")
  (message `/Game/Interaface/BPI_GameMode.IRemoveWorld` _returnvalue (`self.World`))
  (message `/Game/Interaface/BPI_GameMode.IRemoveObstacle` _returnvalue (`|MakeArray` self :!type "Actor Object Reference")))

(event `/Game/Interaface/BPI_Obstacle.IAddWorlds`
  (bind _result (`self.CheckAndSetWorld`))
  (message `/Game/Interaface/BPIW_World.ISetText` (`WidgetComponent.GetWidget` (`self.Widget`)) (`KismetTextLibrary.Conv_StringToText` _result)))

(event `/Game/Interaface/BPI_Obstacle.IUpdateWorld`
  (params (CurrentWorld :type String))
  (`self.HighlightWorld` CurrentWorld)
  (set `self.bIsUpdateWorld` true))

(event `self.Cube.OnComponentBeginOverlap`
  (params (OverlappedComponent :type "PrimitiveComponent Object Reference") (OtherActor :type "Actor Object Reference") (OtherComp :type "PrimitiveComponent Object Reference") (OtherBodyIndex :type Integer) (bFromSweep :type Boolean) (SweepResult :type "HitResult Structure (by ref)"))
  (if (`self.ActorHasTag` OtherActor "Character")
    (message `/Game/Interaface/BPI_HUD.IFinishMenu` (`PlayerController.GetHUD` (`GameplayStatics.GetPlayerController` 0)) true)
    (`GameplayStatics.SetGamePaused` true)
    (`GameplayStatics.PlaySound2D` "/Game/Sound/SFX/SC_Crash.SC_Crash" 1.0 1.0 0.0 null null)))

(event `/Game/Interaface/BPI_Obstacle.IEmpty`
  (bind _returnvalue (`GameplayStatics.GetGameMode`))
  (message `/Game/Interaface/BPIW_World.ISetText` (`WidgetComponent.GetWidget` (`self.Widget`)) "")
  (message `/Game/Interaface/BPI_GameMode.IRemoveWorld` _returnvalue (`self.World`))
  (message `/Game/Interaface/BPI_GameMode.IRemoveObstacle` _returnvalue (`|MakeArray` self :!type "Actor Object Reference")))

(fn `CheckAndSetWorld`
  (returns (Result :type String))
  (locals (World :type String))
  (bind _output_get (`self.SetWorld` :!label _label))
  (set `local.World` _output_get)
  (if (`self.CheckWorld`)
    (return (`local.World`))
    (else
      (goto _label))))

(fn `CheckFirstWorld`
  (params (SourceString :type String))
  (returns (ReturnValue :type Boolean))
  (return (`KismetStringLibrary.NotEqual_StrStr` (`KismetStringLibrary.Left` SourceString 1) (`KismetStringLibrary.Left` (`self.World`) 1))))

(fn `CheckWorld`
  (returns (Value :type Boolean))
  (locals (RetValue :type Boolean))
  (if (`self.LengthWorld` (`self.GetWorlds`))
    (for _array_element (`self.GetWorlds`)
      (bind _output_get (set `local.RetValue` (`self.CheckFirstWorld` _array_element)))
      (if (not _output_get)
        (return (`local.RetValue`))))
    (return (`local.RetValue`))
    (else
      (bind _output_get_2 (set `local.RetValue` true))
      (return _output_get_2))))

(fn `GetLenWorld`
  (params (World :type String))
  (returns (Len :type Integer))
  (return (- (`KismetStringLibrary.Len` World) 1)))

(fn `GetListWorlds`
  (returns (Worlds :type "Array of String"))
  (bind _worlds (message `/Game/Interaface/BPI_Instance.IGetWorlds` (`GameplayStatics.GetGameInstance`) (`self.Index`)))
  (return _worlds))

(fn `GetWorlds`
  (returns (Worlds :type "Array of String"))
  (bind _worlds (message `/Game/Interaface/BPI_GameMode.IGetWorlds` (`GameplayStatics.GetGameMode`)))
  (return _worlds))

(fn `HighlightWorld`
  (params (CurrentWorld :type String))
  (message `/Game/Interaface/BPIW_World.ISetText` (`WidgetComponent.GetWidget` (`self.Widget`)) (`self.SelectionWorld` CurrentWorld CurrentWorld)))

(fn `IGetIsUpdateWorld`
  (returns (Update :type Boolean))
  (return (`self.bIsUpdateWorld`)))

(fn `IGetWorld`
  (returns (World :type String))
  (return (`self.World`)))

(fn `LengthWorld`
  (params (TargetArray :type "Array of String (by ref)"))
  (returns (ReturnValue :type Boolean))
  (return (> (`KismetArrayLibrary.Array_Length` TargetArray) 0)))

(fn `SelectionWorld`
  (params (World :type String) (B :type String))
  (returns (ReturnValue :type Text))
  (bind _world (`self.World`))
  (return (`KismetTextLibrary.Conv_StringToText` (`KismetStringLibrary.Concat_StrStr` (`KismetStringLibrary.Concat_StrStr` "<True>" B "</>") (`KismetStringLibrary.Right` _world (- (`KismetStringLibrary.Len` _world) (+ (`self.GetLenWorld` World) 1)))))))

(fn `SetWorld`
  (returns (Output_Get :type String))
  (bind _worlds (`self.GetListWorlds`))
  (bind _output_get (set `self.World` (`|GetArrayItem` _worlds (`KismetMathLibrary.RandomIntegerInRange` 0 (- (`KismetArrayLibrary.Array_Length` _worlds) 1)))))
  (return _output_get))

(fn `UserConstructionScript`)