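; BP_Obstacle1 is an obstacle that shows a random word (named "World") on its widget, apparently for a typing mechanic.
; It redraws words from the GameInstance list until the first letter differs from every GameMode word.
; Updates show the passed string wrapped in a rich-text highlight tag, with an always-empty remainder.
; Stop zeroes Speed and restores it on a timer, but the movement code is disconnected.
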(event `self.ReceiveTick`
  (params (DeltaSeconds :type "Float (single-precision)")))

(event `self.IStop`
  (set `self.Speed` 0.0)
  (`KismetSystemLibrary.K2_SetTimerDelegate` (delegate `EMove`) 2.0))

(event `EMove`
  (set `self.Speed` 10.0))

(event `self.IAddWorlds`
  (bind _result (`self.CheckAndSetWorld`))
  (message `/Game/Interaface/BPIW_World.ISetText` (`WidgetComponent.GetWidget` (`self.Widget`)) (`KismetTextLibrary.Conv_StringToText` _result)))

(event `self.IUpdateWorld`
  (params (CurrentWorld :type String))
  (`self.HighlightWorld` CurrentWorld))

(fn `CheckAndSetWorld`
  (returns (Result :type String))
  (locals (World :type String))
  (bind _output_get (`self.SetWorld` :!label _label))
  (set `local.World` _output_get)
  (if (`self.CheckWorld`)
    (return (`local.World`))
    (else
      (goto _label))))

(fn `CheckFirstWorld`
  (params (SourceString :type String))
  (returns (ReturnValue :type Boolean))
  (return (`KismetStringLibrary.NotEqual_StrStr` (`KismetStringLibrary.Left` SourceString 1) (`KismetStringLibrary.Left` (`self.World`) 1))))

(fn `CheckWorld`
  (returns (Value :type Boolean))
  (locals (RetValue :type Boolean))
  (if (`self.LengthWorld` (`self.GetWorlds`))
    (for _array_element (`self.GetWorlds`)
      (bind _output_get (set `local.RetValue` (`self.CheckFirstWorld` _array_element)))
      (if (not _output_get)
        (return (`local.RetValue`))))
    (return (`local.RetValue`))
    (else
      (bind _output_get_2 (set `local.RetValue` true))
      (return _output_get_2))))

(fn `GetLenWorld`
  (params (World :type String))
  (returns (Len :type Integer))
  (return (- (`KismetStringLibrary.Len` World) 1)))

(fn `GetListWorlds`
  (returns (Worlds :type "Array of String"))
  (bind _worlds (message `/Game/Interaface/BPI_Instance.IGetWorlds` (`GameplayStatics.GetGameInstance`) 0))
  (return _worlds))

(fn `GetWorlds`
  (returns (Worlds :type "Array of String"))
  (bind _worlds (message `/Game/Interaface/BPI_GameMode.IGetWorlds` (`GameplayStatics.GetGameMode`)))
  (return _worlds))

(fn `HighlightWorld`
  (params (CurrentWorld :type String))
  (message `/Game/Interaface/BPIW_World.ISetText` (`WidgetComponent.GetWidget` (`self.Widget`)) (`self.SelectionWorld` CurrentWorld CurrentWorld)))

(fn `IGetWorld`
  (returns (World :type String))
  (return (`self.World`)))

(fn `LengthWorld`
  (params (TargetArray :type "Array of String (by ref)"))
  (returns (ReturnValue :type Boolean))
  (return (> (`KismetArrayLibrary.Array_Length` TargetArray) 0)))

(fn `SelectionWorld`
  (params (World :type String) (B :type String))
  (returns (ReturnValue :type Text))
  (bind _world (`self.World`))
  (return (`KismetTextLibrary.Conv_StringToText` (`KismetStringLibrary.Concat_StrStr` (`KismetStringLibrary.Concat_StrStr` "<True>" B "</>") (`KismetStringLibrary.Right` _world (- (`KismetStringLibrary.Len` _world) (+ (`self.GetLenWorld` World) 1)))))))

(fn `SetWorld`
  (returns (Output_Get :type String))
  (bind _worlds (`self.GetListWorlds`))
  (bind _output_get (set `self.World` (`|GetArrayItem` _worlds (`KismetMathLibrary.RandomIntegerInRange` 0 (- (`KismetArrayLibrary.Array_Length` _worlds) 1)))))
  (return _output_get))

(fn `UserConstructionScript`)