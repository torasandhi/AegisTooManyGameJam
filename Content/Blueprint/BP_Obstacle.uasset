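; BP_Obstacle is an obstacle that glides toward its mirrored Y position at Z 100, eased over a randomized duration from BeginPlay.
; The IStop event halts the move, then triggers it again after a short delay.
; IAddWorlds picks a random World from the game instance's list via an interface message and prints it, and IGetWorld returns that stored value.
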(event `self.ReceiveBeginPlay`
  (bind (_returnvalue_x _returnvalue_y) (`KismetMathLibrary.BreakVector` (`self.K2_GetActorLocation`)))
  (`KismetSystemLibrary.MoveComponentTo` (`self.DefaultSceneRoot`) (`KismetMathLibrary.MakeVector` _returnvalue_x (* _returnvalue_y -1.0) 100.0) (struct) true true (`KismetMathLibrary.RandomFloatInRange` 8.0 12.0) :!label _label))

(event `/Game/Interaface/BPI_Obstacle.IStop`
  (`|ExecutionSequence`
    (:`then_0`
      (goto _label :!via `Stop`))
    (:`then_1`
      (`KismetSystemLibrary.Delay` 1.0)
      (goto _label))))

(event `/Game/Interaface/BPI_Obstacle.IAddWorlds`
  (bind _worlds (`self.GetWorlds`))
  (bind _output_get (set `self.World` (`|GetArrayItem` _worlds (`KismetMathLibrary.RandomIntegerInRange` 0 (- (`KismetArrayLibrary.Array_Length` _worlds) 1)))))
  (`KismetSystemLibrary.PrintString` _output_get true true (struct :`R` 1.0 :`G` 0.03527 :`A` 1.0) 20.0))

(fn `GetWorlds`
  (returns (Worlds :type "Array of String"))
  (bind _worlds (message `/Game/Interaface/BPI_Instance.IGetWorlds` (`GameplayStatics.GetGameInstance`)))
  (return _worlds))

(fn `IGetWorld`
  (returns (World :type String))
  (return (`self.World`)))

(fn `UserConstructionScript`)