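; BP_Nenek is a character that moves forward automatically, apparently for a runner-style game, and tracks how far it has travelled.
; Each tick, FMove feeds delta-scaled movement input along the forward vector, then updates elapsed time and the X-axis distance from the BeginPlay start location.
; IGetDistance exposes that distance, and CheckObject tests a target for the "Obstacle" tag but is not called in this Blueprint.
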(event `self.ReceiveBeginPlay`
  (set `self.StartLocation` (`self.K2_GetActorLocation`)))

(event `self.ReceiveTick`
  (params (DeltaSeconds :type "Float (single-precision)"))
  (bind _returnvalue_x (`KismetMathLibrary.BreakVector` (`self.K2_GetActorLocation`)))
  (bind _startlocation_x (`KismetMathLibrary.BreakVector` (`self.StartLocation`)))
  (`self.fMove` (`self.MovementSpeed`))
  (set `self.Distance` (`KismetMathLibrary.Vector_Distance` (`KismetMathLibrary.MakeVector` _returnvalue_x) (`KismetMathLibrary.MakeVector` _startlocation_x)))
  (set `self.Time` (+ (`self.Time`) (`GameplayStatics.GetWorldDeltaSeconds`))))

(fn `CheckObject`
  (params (Target :type "Actor Object Reference"))
  (returns (Value :type Boolean))
  (return (`self.ActorHasTag` Target "Obstacle")))

(fn `fMove`
  (params (MoveSpeed :type "Float (double-precision)"))
  (`self.AddMovementInput` (* (`self.GetActorForwardVector`) (* MoveSpeed (`GameplayStatics.GetWorldDeltaSeconds`)))))

(fn `IGetDistance`
  (returns (Distance :type "Float (double-precision)"))
  (return (`self.Distance`)))

(fn `UserConstructionScript`)