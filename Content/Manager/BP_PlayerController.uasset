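; Player controller that captures typed letters for what appears to be a word-typing game.
; Each letter key from A to Z passes its character through InputWorld to the Game Mode's IAddCurrentWorldMessage interface call, while Space Bar sends an empty string.
; Escape calls IPauseMenuMessage on the first player's HUD to bring up the pause menu.
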(event `Key|A`
  (params (Key :type "Key Structure"))
  (:`Pressed`
    (`self.InputWorld` "A")))

(event `Key|E`
  (params (Key :type "Key Structure"))
  (:`Pressed`
    (`self.InputWorld` "E")))

(event `Key|I`
  (params (Key :type "Key Structure"))
  (:`Pressed`
    (`self.InputWorld` "I")))

(event `Key|M`
  (params (Key :type "Key Structure"))
  (:`Pressed`
    (`self.InputWorld` "M")))

(event `Key|Q`
  (params (Key :type "Key Structure"))
  (:`Pressed`
    (`self.InputWorld` "Q")))

(event `Key|U`
  (params (Key :type "Key Structure"))
  (:`Pressed`
    (`self.InputWorld` "U")))

(event `Key|Y`
  (params (Key :type "Key Structure"))
  (:`Pressed`
    (`self.InputWorld` "Y")))

(event `Key|B`
  (params (Key :type "Key Structure"))
  (:`Pressed`
    (`self.InputWorld` "B")))

(event `Key|F`
  (params (Key :type "Key Structure"))
  (:`Pressed`
    (`self.InputWorld` "F")))

(event `Key|J`
  (params (Key :type "Key Structure"))
  (:`Pressed`
    (`self.InputWorld` "J")))

(event `Key|N`
  (params (Key :type "Key Structure"))
  (:`Pressed`
    (`self.InputWorld` "N")))

(event `Key|R`
  (params (Key :type "Key Structure"))
  (:`Pressed`
    (`self.InputWorld` "R")))

(event `Key|V`
  (params (Key :type "Key Structure"))
  (:`Pressed`
    (`self.InputWorld` "V")))

(event `Key|Escape`
  (params (Key :type "Key Structure"))
  (:`Pressed`
    (message `/Game/Interaface/BPI_HUD.IPauseMenu` (`self.GetHUD` (`GameplayStatics.GetPlayerController` 0)) true) ; Pause
  ))

(event `Key|SpaceBar`
  (params (Key :type "Key Structure"))
  (:`Pressed`
    (`self.InputWorld` " ")))

(event `Key|Z`
  (params (Key :type "Key Structure"))
  (:`Pressed`
    (`self.InputWorld` "Z")))

(event `Key|C`
  (params (Key :type "Key Structure"))
  (:`Pressed`
    (`self.InputWorld` "C")))

(event `Key|G`
  (params (Key :type "Key Structure"))
  (:`Pressed`
    (`self.InputWorld` "G")))

(event `Key|K`
  (params (Key :type "Key Structure"))
  (:`Pressed`
    (`self.InputWorld` "K")))

(event `Key|O`
  (params (Key :type "Key Structure"))
  (:`Pressed`
    (`self.InputWorld` "O")))

(event `Key|S`
  (params (Key :type "Key Structure"))
  (:`Pressed`
    (`self.InputWorld` "S")))

(event `Key|W`
  (params (Key :type "Key Structure"))
  (:`Pressed`
    (`self.InputWorld` "W")))

(event `Key|X`
  (params (Key :type "Key Structure"))
  (:`Pressed`
    (`self.InputWorld` "X")))

(event `Key|D`
  (params (Key :type "Key Structure"))
  (:`Pressed`
    (`self.InputWorld` "D")))

(event `Key|H`
  (params (Key :type "Key Structure"))
  (:`Pressed`
    (`self.InputWorld` "H")))

(event `Key|L`
  (params (Key :type "Key Structure"))
  (:`Pressed`
    (`self.InputWorld` "L")))

(event `Key|P`
  (params (Key :type "Key Structure"))
  (:`Pressed`
    (`self.InputWorld` "P")))

(event `Key|T`
  (params (Key :type "Key Structure"))
  (:`Pressed`
    (`self.InputWorld` "T")))

(fn `InputWorld`
  (params (World :type String))
  (message `/Game/Interaface/BPI_GameMode.IAddCurrentWorld` (`GameplayStatics.GetGameMode`) World))

(fn `UserConstructionScript`)