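; Game mode for an endless-road typing game where the player types words shown on obstacles.
; IStart pools six tile types and lays random tiles along X by tag-based length, recycling released tiles back into the road.
; Typed characters lock onto an obstacle by first letter, wrong ones are trimmed, and completed words stop its message and raise the score.
; Older road-building chains remain unwired, leaving the Roads array behind IAddRoadfromPool unfilled.
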(event `self.ReceiveTick`
  (params (DeltaSeconds :type "Float (single-precision)")))

(event `self.ReceiveBeginPlay`)

(event `/Game/Interaface/BPI_GameMode.IStart`
  (for _ (range 11)
    (bind _returnvalue (`|SpawnActorFromClass` "/Game/Blueprint/WorldComponent/BP_Tile_1.BP_Tile_1_C" (`KismetMathLibrary.MakeTransform` (0.0 0.0 10000.0)) "Undefined" "MultiplyWithRoot" null null))
    (`KismetArrayLibrary.Array_Add` (`self.Pool`) _returnvalue)
    (bind _returnvalue_2 (`|SpawnActorFromClass` "/Game/Blueprint/WorldComponent/BP_Tile_2.BP_Tile_2_C" (`KismetMathLibrary.MakeTransform` (0.0 0.0 10000.0)) "Undefined" "MultiplyWithRoot" null null))
    (`KismetArrayLibrary.Array_Add` (`self.Pool`) _returnvalue_2)
    (bind _returnvalue_3 (`|SpawnActorFromClass` "/Game/Blueprint/WorldComponent/BP_Tile_3.BP_Tile_3_C" (`KismetMathLibrary.MakeTransform` (0.0 0.0 10000.0)) "Undefined" "MultiplyWithRoot" null null))
    (`KismetArrayLibrary.Array_Add` (`self.Pool`) _returnvalue_3)
    (bind _returnvalue_4 (`|SpawnActorFromClass` "/Game/Blueprint/WorldComponent/BP_Tile_4.BP_Tile_4_C" (`KismetMathLibrary.MakeTransform` (0.0 0.0 10000.0)) "Undefined" "MultiplyWithRoot" null null))
    (`KismetArrayLibrary.Array_Add` (`self.Pool`) _returnvalue_4)
    (bind _returnvalue_5 (`|SpawnActorFromClass` "/Game/Blueprint/WorldComponent/BP_Tile_5.BP_Tile_5_C" (`KismetMathLibrary.MakeTransform` (0.0 0.0 10000.0)) "Undefined" "MultiplyWithRoot" null null))
    (`KismetArrayLibrary.Array_Add` (`self.Pool`) _returnvalue_5)
    (bind _returnvalue_6 (`|SpawnActorFromClass` "/Game/Blueprint/WorldComponent/BP_Tile_6.BP_Tile_6_C" (`KismetMathLibrary.MakeTransform` (0.0 0.0 10000.0)) "Undefined" "MultiplyWithRoot" null null))
    (`KismetArrayLibrary.Array_Add` (`self.Pool`) _returnvalue_6))
  (for _ (range 21)
    (`self.SpawnRoad` 1)))

(event `/Game/Interaface/BPI_GameMode.IAddObstacle`
  (params (Obstacle :type "Object Object Reference"))
  (`KismetArrayLibrary.Array_Add` (`self.Obstacles`) Obstacle)
  (`self.AddWorld`)
  (set `self.CurrentWorlds` (`self.Worlds`)))

(event `/Game/Interaface/BPI_GameMode.IRemoveWorld`
  (params (World :type String))
  (`KismetArrayLibrary.Array_RemoveItem` (`self.Worlds`) World)
  (set `self.CurrentWorld` "")
  (set `self.TargetWorld` "")
  (set `self.TargetObstacle` null))

(event `/Game/Interaface/BPI_GameMode.IAddCurrentWorld`
  (params (World :type String))
  (set `self.CurrentWorld` (`KismetStringLibrary.Concat_StrStr` (`self.CurrentWorld`) World))
  (`self.FindWord`)
  (`self.CorrectWorlds`))

(event `/Game/Interaface/BPI_GameMode.IAddRoadFromPool`
  (`self.ExtendRoads`))

(event `/Game/Interaface/BPI_GameMode.IRemoveArray`
  (params (Actor :type "Actor Object Reference"))
  (`KismetArrayLibrary.Array_RemoveItem` (`self.Spawned`) Actor)
  (`KismetArrayLibrary.Array_Add` (`self.Pool`) Actor)
  (`self.SpawnRoad` 5))

(event `/Game/Interaface/BPI_GameMode.IRemoveObstacle`
  (params (Obstacles :type "Array of Actor Object Reference (by ref)"))
  (for _array_element Obstacles
    (`KismetArrayLibrary.Array_RemoveItem` (`self.Obstacles`) _array_element)))

(fn `AddRoads`
  (bind _returnvalue (`|SpawnActorFromClass` "/Game/Blueprint/WorldComponent/Road.Road_C" (`self.AttachRoadLocation`) "Undefined" "MultiplyWithRoot" null null))
  (bind _returnvalue_2 (`/Game/Blueprint/WorldComponent/Road.GetAttachLocation` _returnvalue))
  (set `self.AttachRoadLocation` _returnvalue_2)
  (`KismetArrayLibrary.Array_Add` (`self.Roads`) _returnvalue))

(fn `AddWorld`
  (`KismetArrayLibrary.Array_Clear` (`self.Worlds`))
  (for _array_element (`self.Obstacles`)
    (bind _world (message `/Game/Interaface/BPI_Obstacle.IGetWorld` _array_element))
    (`KismetArrayLibrary.Array_Add` (`self.Worlds`) _world)))

(fn `BuildRoad`
  (`self.K2_SetActorLocation` (`self.RandomTypeComponent`) (`self.LastPosition`) false false)
  (`KismetArrayLibrary.Array_Add` (`self.Spawned`) (`|GetArrayItem` (`self.Components`)))
  (set `self.LastPosition` (+ (`self.LastPosition`) (`self.Get Last Actor`))))

(fn `CheckingWorlds`
  (returns (Value :type Boolean))
  (bind _len (`self.LenCurrentWorld`))
  (return (`KismetStringLibrary.EqualEqual_StrStr` (`KismetStringLibrary.Mid` (`self.TargetWorld`) _len 1) (`KismetStringLibrary.Mid` (`self.CurrentWorld`) _len 1))))

(fn `CheckSetence`
  (returns (Value :type Boolean))
  (return (`KismetStringLibrary.EqualEqual_StrStr` (`self.CurrentWorld`) (`self.TargetWorld`))))

(fn `CorrectWorlds`
  (if (`self.CheckingWorlds`)
    (message `/Game/Interaface/BPI_Obstacle.IUpdateWorld` (`self.TargetObstacle`) (`self.CurrentWorld`))
    (if (`self.CheckSetence`)
      (message `/Game/Interaface/BPI_Obstacle.IStop` (`self.TargetObstacle`))
      (`KismetArrayLibrary.Array_Remove` (`self.CurrentWorlds`) (`self.Index`))
      (set `self.CurrentWorld` "")
      (set `self.Index` 0)
      (set `self.TargetObstacle` null)
      (set `self.TotalCorrectWorlds` (+ (`self.TotalCorrectWorlds`) 1)))
    (else
      (`self.WorldCorrection`))))

(fn `ExtendRoads`
  (bind _roads (`self.Roads`))
  (bind _output (`|GetArrayItem` _roads))
  (bind _returnvalue (`/Game/Blueprint/WorldComponent/Road.GetAttachLocation` (`|GetArrayItem` _roads (`KismetArrayLibrary.Array_LastIndex` _roads))))
  (`self.K2_SetActorLocation` _output (.location _returnvalue) false false)
  (bind _returnvalue_2 (`KismetArrayLibrary.Array_RemoveItem` _roads _output))
  (if _returnvalue_2
    (`KismetArrayLibrary.Array_Add` _roads _output)
    (return)))

(fn `FindWord`
  (locals (CorrectWorld :type String))
  (for (_array_element _array_index) (`self.CurrentWorlds`)
    (if (and (`KismetStringLibrary.EqualEqual_StrStr` (`KismetStringLibrary.Left` _array_element 1) (`KismetStringLibrary.Left` (`self.CurrentWorld`) 1)) (not (`KismetSystemLibrary.IsValid` (`self.TargetObstacle`))))
      (set `self.TargetWorld` _array_element)
      (set `self.Index` _array_index)
      (set `self.TargetObstacle` (`|GetArrayItem` (`self.Obstacles`) (`self.Index`))))))

(fn `Get Last Actor`
  (returns (Value :type "Vector Structure"))
  (bind _spawned (`self.Spawned`))
  (switch `name` (`|GetArrayItem` (`Actor.Tags` (`|GetArrayItem` _spawned (- (`KismetArrayLibrary.Array_Length` _spawned) 1))))
    (:`Road_1`
      _)
    (:`Road_2`
      (return (200.0 0.0 0.0)))
    (:`Road_3`
      (return (300.0 0.0 0.0)))
    (:`Ground_1`
      _)
    (:`Ground_2`
      (return (200.0 0.0 0.0))))
  (return (100.0 0.0 0.0)))

(fn `GetLengthPool`
  (params (B :type Integer))
  (returns (Value :type Integer))
  (return (- (`KismetArrayLibrary.Array_Length` (`self.Pool`)) B)))

(fn `GetRoad`
  (params (B :type Integer))
  (returns (Road :type "Actor Object Reference"))
  (locals (TempActor :type "Actor Object Reference"))
  (bind _tempactor (`local.TempActor`))
  (bind _output_get (set `local.TempActor` (`|GetArrayItem` (`self.Pool`) (`KismetMathLibrary.RandomIntegerInRange` 0 (`self.GetLengthPool` B)))))
  (`KismetArrayLibrary.Array_RemoveItem` (`self.Pool`) _output_get)
  (`KismetArrayLibrary.Array_Add` (`self.Spawned`) _tempactor)
  (return _tempactor))

(fn `GetSameWorld`
  (returns (Index :type Integer))
  (locals (CurrentIndex :type Integer) (Booll :type Boolean))
  (for (_array_element _array_index) (`self.Obstacles`)
    (bind _world (message `/Game/Interaface/BPI_Obstacle.IGetWorld` _array_element))
    (if (and (`KismetStringLibrary.EqualEqual_StrStr` (`KismetStringLibrary.Left` _world (`self.LenCurrentWorld`)) (`KismetStringLibrary.Left` (`self.TargetWorld`) (`self.LenCurrentWorld`))) (not (`local.Booll`)))
      (set `local.CurrentIndex` _array_index)
      (set `local.Booll` true)))
  (return (`local.CurrentIndex`)))

(fn `IGetCorrectWords`
  (returns (CorrectWords :type Integer))
  (return (`self.TotalCorrectWorlds`)))

(fn `IGetWorld`
  (returns (World :type String))
  (return (`|GetArrayItem` (`self.Worlds`))))

(fn `IGetWorlds`
  (returns (Worlds :type "Array of String"))
  (return (`self.CurrentWorlds`)))

(fn `LenCurrentWorld`
  (returns (Len :type Integer))
  (return (- (`KismetStringLibrary.Len` (`self.CurrentWorld`)) 1)))

(fn `RandomTypeComponent`
  (returns (Value :type "Actor Object Reference"))
  (bind _output (`|GetArrayItem` (`self.Components`) (`KismetMathLibrary.RandomIntegerInRange` 0 3)))
  (`KismetArrayLibrary.Array_Add` (`self.Spawned`) _output)
  (return _output))

(fn `SpawnRoad`
  (params (B :type Integer))
  (locals (Length :type "Vector Structure"))
  (bind _spawned (`self.Spawned`))
  (`self.K2_SetActorLocation` (`self.GetRoad` B) (`self.LastPosition`) false false)
  (`|ExecutionSequence`
    (:`then_0`
      (switch `name` (`|GetArrayItem` (`Actor.Tags` (`|GetArrayItem` _spawned (- (`KismetArrayLibrary.Array_Length` _spawned) 1))))
        (:`7`
          (set `local.Length` (700.0 0.0 0.0)))
        (:`9`
          (set `local.Length` (900.0 0.0 0.0)))
        (:`5`
          (set `local.Length` (500.0 0.0 0.0)))
        (:`6`
          (set `local.Length` (600.0 0.0 0.0)))
        (:`11`
          (set `local.Length` (1100.0 0.0 0.0)))))
    (:`then_1`
      (set `self.LastPosition` (+ (`self.LastPosition`) (`local.Length`))))))

(fn `UserConstructionScript`)

(fn `WorldCorrection`
  (set `self.CurrentWorld` (`KismetStringLibrary.Left` (`self.CurrentWorld`) (`self.LenCurrentWorld`))))